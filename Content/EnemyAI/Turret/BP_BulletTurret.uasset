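; Bullet actor for the enemy turret that damages the player character on contact.
; A capsule hit that casts to BP_Character applies the Damage value and destroys the bullet; other hits are ignored.
; UpdatePlayerPosition returns the location of the first actor found by a class search, stored as PlayerVector, but no graph here calls it.
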(event `self.CapsuleComponent.OnComponentHit`
  (params (HitComponent :type "PrimitiveComponent Object Reference") (OtherActor :type "Actor Object Reference") (OtherComp :type "PrimitiveComponent Object Reference") (NormalImpulse :type "Vector Structure") (Hit :type "HitResult Structure (by ref)"))
  (bind _asbp_character (cast `/Game/Blueprints/Player/BP_Character` OtherActor))
  (`GameplayStatics.ApplyDamage` _asbp_character (`self.damage`))
  (`self.K2_DestroyActor`))

(fn `UpdatePlayerPosition`
  (returns (PlayerLocation :type "Vector Structure"))
  (bind _outactors (`GameplayStatics.GetAllActorsOfClass` null))
  (bind _output (`|GetArrayItem` _outactors))
  (`/Engine/EditorBlueprintResources/StandardMacros.IsValid` _output
    (:`Is Valid`
      (bind _output_get (set `self.PlayerVector` (`self.K2_GetActorLocation` _output)))
      (return _output_get))))

(fn `UserConstructionScript`)