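; BP_Turret is an AI turret that spots the player character class, turns toward it and fires.
; BeginPlay sets the PawnSensing sight radius from the cannon range.
; Each sighting of a BP_Character snaps the whole actor to face it, then a fire-rate Delay gates the shot.
; After the delay it spawns BP_BulletTurret at the Arrow transform with the cannon damage and plays the Canon sound.
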(event `self.ReceiveBeginPlay`
  (set `PawnSensingComponent.SightRadius` (`self.CannonRange`) (`self.PawnSensing`)))

(event `self.PawnSensing.OnSeePawn`
  (params (Pawn :type "Pawn Object Reference"))
  (cast `/Game/Blueprints/Player/BP_Character` Pawn)
  (`self.K2_SetActorRotation` (`KismetMathLibrary.FindLookAtRotation` (`self.K2_GetActorLocation`) (`self.K2_GetActorLocation` Pawn)))
  (`KismetSystemLibrary.Delay` (`self.CannonFireRate`))
  (`|SpawnActorFromClass` "/Game/AI/Turret/BP_BulletTurret.BP_BulletTurret_C" (`SceneComponent.K2_GetComponentToWorld` (`self.Arrow`)) "Undefined" "MultiplyWithRoot" null (`self.CannonDamage`) null)
  (`AudioComponent.Play` (`self.Canon`) 0.0))

(fn `UserConstructionScript`)