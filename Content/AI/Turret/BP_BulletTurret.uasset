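; BP_BulletTurret is a turret bullet that damages the player character on impact.
; Its Hit event calls DealDamage when it strikes BP_Character, which applies Damage to the first BP_Character in the level and destroys the bullet.
; Any other impact destroys it immediately.
; An UpdatePlayerPosition helper returns the location of the first actor from a class search, but nothing here calls it.
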(event `self.ReceiveHit`
  (params (MyComp :type "PrimitiveComponent Object Reference") (Other :type "Actor Object Reference") (OtherComp :type "PrimitiveComponent Object Reference") (bSelfMoved :type Boolean) (HitLocation :type "Vector Structure") (HitNormal :type "Vector Structure") (NormalImpulse :type "Vector Structure") (Hit :type "HitResult Structure (by ref)"))
  (if (== Other "/Game/Blueprints/Player/BP_Character.BP_Character")
    (`self.DealDamage`)
    (else
      (`self.K2_DestroyActor`))))

(event `self.DealDamage`
  ;[1 1 1] Deal damage
  (bind _outactors (`GameplayStatics.GetAllActorsOfClass` "/Game/Blueprints/Player/BP_Character.BP_Character_C"))
  (`GameplayStatics.ApplyDamage` (`|GetArrayItem` _outactors) (`self.damage`) null self)
  (`self.K2_DestroyActor`))

(fn `UpdatePlayerPosition`
  (returns (PlayerLocation :type "Vector Structure"))
  (bind _outactors (`GameplayStatics.GetAllActorsOfClass` null))
  (bind _output (`|GetArrayItem` _outactors))
  (`/Engine/EditorBlueprintResources/StandardMacros.IsValid` _output
    (:`Is Valid`
      (bind _output_get (set `self.PlayerVector` (`self.K2_GetActorLocation` _output)))
      (return _output_get))))

(fn `UserConstructionScript`)