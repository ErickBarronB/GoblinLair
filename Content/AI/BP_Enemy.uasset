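; BP_Enemy is an enemy actor that damages the player at close range and destroys itself when its health runs out.
; Each Tick fetches the first BP_Character's location and, within DistanceToAttack, starts an AttackRate Delay that paces DealDamage without rechecking range.
; DealDamage applies damage to that character, while TakeDamage lowers Health, which Tick polls for death.
; It contains no movement logic, and a Health debug print is left unconnected.
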(event `self.ReceiveTick`
  (params (DeltaSeconds :type "Float (single-precision)"))
  (`|ExecutionSequence`
    (:`then_0`
      (bind _playerlocation (`self.UpdatePlayerPosition`))
      (if (<= (`KismetMathLibrary.Vector_Distance` (`self.K2_GetActorLocation`) _playerlocation) (`self.DistanceToAttack`))
        (`KismetSystemLibrary.Delay` (`self.AttackRate`))
        (`self.DealDamage`)))
    (:`then_1`
      (if (<= (`self.Health`) 0.0)
        (`self.K2_DestroyActor`)))))

(event `self.DealDamage`
  (bind _outactors (`GameplayStatics.GetAllActorsOfClass` "/Game/Blueprints/Player/BP_Character.BP_Character_C"))
  (`GameplayStatics.ApplyDamage` (`|GetArrayItem` _outactors) (`self.damage`) null self))

(event `/Game/AI/IEnemy.TakeDamage`
  (params (Damage :type "Float (double-precision)"))
  (set `self.Health` (- (`self.Health`) Damage)))

(fn `UpdatePlayerPosition`
  (returns (PlayerLocation :type "Vector Structure"))
  (bind _outactors (`GameplayStatics.GetAllActorsOfClass` "/Game/Blueprints/Player/BP_Character.BP_Character_C"))
  (bind _output_get (set `self.PlayerVector` (`self.K2_GetActorLocation` (`|GetArrayItem` _outactors))))
  (return _output_get))

(fn `UserConstructionScript`)