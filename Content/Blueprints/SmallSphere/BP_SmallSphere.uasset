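; BP_SmallSphere is an actor that wanders through the world, constantly moving and turning on its own.
; BeginPlay picks a random rotator once and stores it as a per-second rotation rate.
; Each Tick moves the actor along its forward vector without sweeping, then applies that rotation, so its path curves.
; Rotation scales with delta time, while movement adds Speed per frame and depends on frame rate.
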(event `self.ReceiveBeginPlay`
  (`self.InitRotation`))

(event `self.ReceiveTick`
  (params (DeltaSeconds :type "Float (single-precision)"))
  (`self.UpdateMovement`)
  (`self.UpdateRotation` DeltaSeconds))

(fn `InitRotation`
  (set `self.Delta Rotation` (`KismetMathLibrary.RandomRotator` false)))

(fn `UpdateMovement`
  (`self.K2_AddActorWorldOffset` (* (`self.GetActorForwardVector`) (`self.Speed`))))

(fn `UpdateRotation`
  (params (B :type "Float (single-precision)"))
  (`self.K2_AddActorWorldRotation` (* (`self.Delta Rotation`) B)))

(fn `UserConstructionScript`)