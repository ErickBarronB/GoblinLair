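; BP_Book is a book weapon that fires BP_BookProjectile magic projectiles.
; FireWeapon spawns the projectile at the ProjectileLaunch transform, passing MagicSpeed as its travel speed, then clears CanFire.
; Tick restores CanFire through a one-second Delay, forming a cooldown.
; Each fire call also runs a debug-drawn camera line trace, even during cooldown, but its result is unused.
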(event `self.ReceiveTick`
  (params (DeltaSeconds :type "Float (single-precision)"))
  (if (== (`self.canFire`) false)
    (`KismetSystemLibrary.Delay` 1.0)
    (set `self.canFire` true)))

(event `self.FireWeapon`
  (`KismetSystemLibrary.LineTraceSingle` :`Start` (`PlayerCameraManager.GetCameraLocation` (`GameplayStatics.GetPlayerCameraManager` 0)) :`End` (`self.RaycastEndPosition`) :`TraceChannel` "TraceTypeQuery1" :`DrawDebugType` "ForDuration")
  (if (== (`self.canFire`) true)
    (`|SpawnActorFromClass` "/Game/Blueprints/Weapons/Weapons/Projectile/BP_BookProjectile.BP_BookProjectile_C" (`SceneComponent.K2_GetComponentToWorld` (`self.ProjectileLaunch`)) "AlwaysSpawn" "MultiplyWithRoot" null (`self.MagicSpeed`) null)
    (set `self.canFire` false)))

(fn `UserConstructionScript`
  (`parent.UserConstructionScript`))