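; BP_BookProjectile is a magic book weapon projectile that steers with the player's view and hits AI enemies.
; On spawn it plays the MagicSpell sound through the player pawn's AudioComponent.
; Each tick, FollowCursor offsets it along the current camera forward vector by TravelSpeed, without sweep or delta-time scaling.
; Component hits on an AI_Enemy pass the projectile to that enemy's ProjectileHit.
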(event `self.ReceiveBeginPlay`
  (bind _returnvalue (`self.GetComponentByClass` (`GameplayStatics.GetPlayerPawn` 0) "/Script/Engine.AudioComponent"))
  ;[1 1 1] Plays sound when spawn
  (`AudioComponent.SetSound` _returnvalue "/Game/Audio/MagicSpell.MagicSpell")
  (`AudioComponent.Play` _returnvalue 0.0))

(event `self.ReceiveTick`
  (params (DeltaSeconds :type "Float (single-precision)"))
  (`self.Follow Cursor`))

(event `self.Projectile.OnComponentHit`
  (params (HitComponent :type "PrimitiveComponent Object Reference") (OtherActor :type "Actor Object Reference") (OtherComp :type "PrimitiveComponent Object Reference") (NormalImpulse :type "Vector Structure") (Hit :type "HitResult Structure (by ref)"))
  (bind _asai_enemy (cast `/Game/EnemyAI/AI_Enemy` OtherActor))
  (`/Game/EnemyAI/AI_Enemy.Projectile Hit` _asai_enemy self))

(fn `Follow Cursor`
  (`self.K2_AddActorWorldOffset` (* (`KismetMathLibrary.GetForwardVector` (`PlayerCameraManager.GetCameraRotation` (`PlayerController.PlayerCameraManager` (`GameplayStatics.GetPlayerController` 0)))) (`self.TravelSpeed`))))

(fn `UserConstructionScript`)