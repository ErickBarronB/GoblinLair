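; BP_BaseWeapon is a base weapon Blueprint that fires a camera-aimed hitscan shot.
; FireWeapon sphere-traces on Visibility from the player 0 camera to a point WeaponRange along its forward vector, ignoring all weapon actors.
; Hit actors implementing IEnemy receive TakeDamageMessage with Damage; otherwise it prints the hit actor's name.
; The trace draws persistent debug shapes, and a LineTraceByChannel node is left unconnected.
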(event `FireWeapon`
  (bind _outactors (`GameplayStatics.GetAllActorsOfClass` "BP_BaseWeapon_C"))
  (bind _outhit (`KismetSystemLibrary.SphereTraceSingle` (`PlayerCameraManager.GetCameraLocation` (`GameplayStatics.GetPlayerCameraManager` 0)) (`self.RaycastEndPosition`) 0.0 "TraceTypeQuery1" false _outactors "Persistent"))
  (if (`KismetSystemLibrary.DoesImplementInterface` (`.HitActor` (`GameplayStatics.BreakHitResult` _outhit)) "/Game/AI/IEnemy.IEnemy_C")
    (message `/Game/AI/IEnemy.TakeDamage` (`.HitActor` (`GameplayStatics.BreakHitResult` _outhit)) (`self.Damage`))
    (else
      (`KismetSystemLibrary.PrintString` (`KismetSystemLibrary.GetDisplayName` (`.HitActor` (`GameplayStatics.BreakHitResult` _outhit)))))))

(fn `RaycastEndPosition`
  (returns (ReturnValue :type "Vector Structure"))
  (return (+ (`PlayerCameraManager.GetCameraLocation` (`GameplayStatics.GetPlayerCameraManager` 0)) (* (`KismetMathLibrary.GetForwardVector` (`PlayerCameraManager.GetCameraRotation` (`GameplayStatics.GetPlayerCameraManager` 0))) (`self.WeaponRange`)))))

(fn `UserConstructionScript`)