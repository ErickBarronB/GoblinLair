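; BP_SmallSphere is an interactable actor that spins in place and opens a level when interacted with.
; On BeginPlay it picks a random rotator without roll, then applies it scaled by delta time each Tick for frame-rate-independent world rotation.
; The Interact event loads the level referenced by its Level variable through Open Level by Object Reference.
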(event `self.ReceiveBeginPlay`
  ;[1 1 1] Rotation/Movement
  (`self.InitRotation`))

(event `self.ReceiveTick`
  (params (DeltaSeconds :type "Float (single-precision)"))
  ;[1 1 1] Rotation/Movement
  (`self.UpdateRotation` DeltaSeconds))

(event `/Game/Blueprints/Interface_Interactables.Interact`
  ;[1 1 1] Pick Up
  (`GameplayStatics.OpenLevelBySoftObjectPtr` (`self.Level`)))

(fn `InitRotation`
  (set `self.Delta Rotation` (`KismetMathLibrary.RandomRotator` false)))

(fn `UpdateRotation`
  (params (B :type "Float (single-precision)"))
  (`self.K2_AddActorWorldRotation` (* (`self.Delta Rotation`) B)))

(fn `UserConstructionScript`)