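; Interactable door Blueprint that swings open or shut each time it receives the Interact event.
; A FlipFlop alternates between the OpenDoor and CloseDoor functions.
; Each function snaps the Scene component's relative rotation between a quarter-turn yaw and zero, with no animated transition.
; Debug strings print the object name and the open or close action.
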(event `/Game/Blueprints/Interface_Interactables.Interact`
  (`KismetSystemLibrary.PrintString` (`KismetStringLibrary.Concat_StrStr` (`KismetSystemLibrary.GetObjectName` self) " is" " Interactable"))
  (`/Engine/EditorBlueprintResources/StandardMacros.FlipFlop`
    (:`A`
      (`self.Open Door`))
    (:`B`
      (`self.Close Door`))))

(fn `Close Door`
  (`KismetSystemLibrary.PrintString` "close")
  (`SceneComponent.K2_SetRelativeRotation` (`self.Scene`) (`KismetMathLibrary.MakeRotator` 0.0) false false))

(fn `Open Door`
  (`KismetSystemLibrary.PrintString` "open")
  (`SceneComponent.K2_SetRelativeRotation` (`self.Scene`) (`KismetMathLibrary.MakeRotator` 0.0 0.0 -90.0) false false))

(fn `UserConstructionScript`)