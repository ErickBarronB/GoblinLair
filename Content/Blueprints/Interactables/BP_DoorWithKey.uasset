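; BP_DoorWithKey is an interactable door that only opens or closes when its Haskey flag is set.
; Interact checks the flag and uses a FlipFlop to alternate between OpenDoor and CloseDoor, or prints a message that a key is needed.
; Both functions snap the Scene component's relative rotation between a quarter-turn yaw and zero, with no animation.
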(event `/Game/Blueprints/Interface_Interactables.Interact`
  (if (`self.haskey`)
    (`/Engine/EditorBlueprintResources/StandardMacros.FlipFlop`
      (:`A`
        (`self.Open Door`))
      (:`B`
        (`self.Close Door`)))
    (else
      (`KismetSystemLibrary.PrintString` "You need a Key"))))

(fn `Close Door`
  (`SceneComponent.K2_SetRelativeRotation` (`self.Scene`) (`KismetMathLibrary.MakeRotator` 0.0) false false))

(fn `Open Door`
  (`SceneComponent.K2_SetRelativeRotation` (`self.Scene`) (`KismetMathLibrary.MakeRotator` 0.0 0.0 -90.0) false false))

(fn `UserConstructionScript`)